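; BP_SmartNPC_Base is a base NPC that moves in response to parsed commands from the game instance's GPT manager.
; It binds to the manager's parsed-command event shortly after BeginPlay.
; For "move" commands, it matches the target against StaticMeshActor object names and against room names on either side of the current room's connected doors.
; Matches become CurrentTarget and are approached with SimpleMoveToLocation.
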(event `self.ReceiveBeginPlay`
  (`KismetSystemLibrary.Delay` 0.1)
  (bind _asglobal_game_instance (cast `GlobalGameInstance` (`GameplayStatics.GetGameInstance`))
    (:`then`
      (bind _returnvalue (`GlobalGameInstance.GetGPTManager` _asglobal_game_instance))
      (add `GPTManager.OnParsedCommand` _returnvalue (delegate `OnParsedCommand_事件`)))
    (:`CastFailed`
      (`KismetSystemLibrary.PrintString` "CAST TO INSTANCE FAILED!"))))

(event `OnParsedCommand_事件`
  (params (Command :type "ParsedCommand Structure (by ref)"))
  ;[1 1 1] 首先寻找目标（Target）
  (if (`KismetStringLibrary.EqualEqual_StrStr` Command_Action "move")
    (bind _outactors (`GameplayStatics.GetAllActorsOfClass` "/Script/Engine.StaticMeshActor"))
    (for _array_element _outactors
      (if (`KismetStringLibrary.EqualEqual_StrStr` Command_Target (`KismetSystemLibrary.GetObjectName` _array_element))
        (`KismetSystemLibrary.PrintString` "FOUND!")
        (bind _output_get (set `self.CurrentTarget` _array_element))
        (`|ExecutionSequence`
          (:`then_0`
            (break))
          (:`then_1`
            (`AIBlueprintHelperLibrary.SimpleMoveToLocation` (`self.GetController` self) (`self.K2_GetActorLocation` _output_get))))))
    ;[1 1 1] 当前NPC 的房间，检查所有链接的门
    (for _array_element_2 (`/Game/MyContent/RoomTriggerBox/Base_RoomTriggerBox.ConnectedDoors` (`self.CurrentRoom`))
      (bind _rooma (`/Game/MyContent/DoorActor/Base_DoorActor.RoomA` _array_element_2))
      ;[1 1 1] 先看第一个房间是不是我们的目标
      (if (`KismetStringLibrary.EqualEqual_StrStr` Command_Target (`/Game/MyContent/RoomTriggerBox/Base_RoomTriggerBox.RoomName` _rooma))
        (set `self.CurrentTarget` _rooma)
        (`KismetSystemLibrary.PrintString` "FOUND!" :!label _label)
        (`|ExecutionSequence`
          (:`then_0`
            (break))
          (:`then_1`
            (`AIBlueprintHelperLibrary.SimpleMoveToLocation` (`self.GetController` self) (`self.K2_GetActorLocation` (`self.CurrentTarget`)))))
        (else
          (bind _roomb (`/Game/MyContent/DoorActor/Base_DoorActor.RoomB` _array_element_2))
          ;[1 1 1] 再看第二个房间
          (if (`KismetSystemLibrary.IsValid` _roomb)
            (if (`KismetStringLibrary.EqualEqual_StrStr` Command_Target (`/Game/MyContent/RoomTriggerBox/Base_RoomTriggerBox.RoomName` _roomb))
              (set `self.CurrentTarget` _roomb)
              (goto _label))))))
    (`KismetSystemLibrary.PrintString` "NOT FOUND")))

(fn `UserConstructionScript`)