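; Player-possessable room camera that lets the player look around with yaw and pitch input.
; On BeginPlay it caches BP_StaticCamController and, if active, shows its room name and registers itself as the current camera.
; A separate event updates the room-name hint widget from a given camera.
; Angle clamping, chat UI, and trace-based switching between cameras remain as disconnected, unexecuted logic.
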(event `self.ReceiveBeginPlay`
  (bind _asbp_static_cam_controller (cast `/Game/MyContent/BP_StaticCamController` (`GameplayStatics.GetPlayerController` 0)))
  (bind _output_get (set `self.StaticCamController` _asbp_static_cam_controller))
  (if (`self.isCurrentActive`)
    (`/Game/MyContent/BP_StaticCamController.SetCameraLocationText` _output_get (`KismetTextLibrary.Conv_StringToText` (`/Game/MyContent/RoomTriggerBox/Base_RoomTriggerBox.RoomName` (`self.Room`))))
    ; 设置当前相机对象
    (bind _asbp_static_cam_controller_2 (cast `/Game/MyContent/BP_StaticCamController` (`GameplayStatics.GetPlayerController` 0)))
    (set `/Game/MyContent/BP_StaticCamController.CurrentCamera` self _asbp_static_cam_controller_2)))

(event `self.ReceiveTick`
  (params (DeltaSeconds :type "Float (single-precision)"))
  (`self.AddControllerYawInput` (`self.GetInputAxisKeyValue`))
  (`self.AddControllerPitchInput` (* (`self.GetInputAxisKeyValue`) -1.0))
  (if (`self.ChangeViewUIShown`)
    _))

(event `ChangeRoomNameHint`
  (params (CurrentCameraObj :type "/Game/MyContent/BP_Player_Camera Object Reference"))
  (`TextBlock.SetText` (`/Game/MyContent/WBP_RoomHintUI.RoomHintText` (`self.RoomNameHintUI`)) (`KismetTextLibrary.Conv_StringToText` (`/Game/MyContent/RoomTriggerBox/Base_RoomTriggerBox.RoomName` (`/Game/MyContent/BP_Player_Camera.Room` CurrentCameraObj)))))

(event `Key|R`
  (params (Key :type "Key Structure"))
  ;[1 1 1] 按下R之后的逻辑
)

(event `ShowChangeViewHintWidget`
  (params (Show :type Boolean)))

(event `Key|F`
  (params (Key :type "Key Structure")))

(fn `UserConstructionScript`)