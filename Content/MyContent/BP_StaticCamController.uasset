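; Static camera controller that lets the player hop between BP_Player_Camera views and open a chat UI.
; A Delay-throttled Tick traces from screen center; aiming at another camera shows a hint and enables R to blend the view, then possess it.
; F opens the chat widget with UI-only input.
; Events set the room-name label, add chat history and send it to the LLM via the game instance's GPT manager.
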(event `self.ReceiveBeginPlay`)

(event `SetCameraLocationText`
  (params (CameraLocation :type Text))
  ;[1 1 1] 切换摄像机右上角的地点名称
  (`/Engine/EditorBlueprintResources/StandardMacros.IsValid` (`self.RoomNameHintUI`)
    (:`Is Valid`
      _)
    (:`Is Not Valid`
      (bind _returnvalue (`|CreateWidget` "/Game/MyContent/WBP_RoomHintUI.WBP_RoomHintUI_C"))
      (bind _output_get (set `self.RoomNameHintUI` _returnvalue))
      (`UserWidget.AddToViewport` _output_get 0)
      (`Widget.SetVisibility` (`/Game/MyContent/WBP_RoomHintUI.RoomHintText` _output_get) "Visible")))
  (bind _output_get_2 (set `self.CameraLocationText` CameraLocation))
  (`TextBlock.SetText` (`/Game/MyContent/WBP_RoomHintUI.RoomHintText` (`self.RoomNameHintUI`)) _output_get_2))

(event `ShowChangeViewHint`
  (params (Show :type Boolean))
  (bind _changeviewhintui (`self.ChangeViewHintUI`))
  ; 提示“按R切换摄像头”
  (if Show
    (`/Engine/EditorBlueprintResources/StandardMacros.IsValid` _changeviewhintui
      (:`Is Valid`
        _)
      (:`Is Not Valid`
        (bind _returnvalue (`|CreateWidget` "/Game/MyContent/WBP_ChangeViewHintUI.WBP_ChangeViewHintUI_C"))
        (bind _output_get (set `self.ChangeViewHintUI` _returnvalue))
        (`UserWidget.AddToViewport` _output_get 0)))
    (`Widget.SetVisibility` _changeviewhintui "Visible")
    (set `self.CanChangeCamera` true)
    (else
      (`/Engine/EditorBlueprintResources/StandardMacros.IsValid` _changeviewhintui
        (:`Is Valid`
          (`Widget.SetVisibility` _changeviewhintui "Hidden"))
        (:`Is Not Valid`
          _))
      (set `self.CanChangeCamera` false))))

(event `self.ReceiveTick`
  (params (DeltaSeconds :type "Float (single-precision)"))
  (bind (_returnvalue_x _returnvalue_y) (`KismetMathLibrary.BreakVector2D` (`WidgetLayoutLibrary.GetViewportSize`)))
  (bind _currentcamera (`self.CurrentCamera`))
  (bind (_worldposition _worlddirection) (`GameplayStatics.DeprojectScreenToWorld` (`GameplayStatics.GetPlayerController` 0) (`KismetMathLibrary.MakeVector2D` (* _returnvalue_x 0.5) (* _returnvalue_y 0.5))))
  ; 检测是否瞄准另外一个摄像头
  (`KismetSystemLibrary.Delay` 0.5)
  (if (`KismetSystemLibrary.IsValid` _currentcamera)
    (bind _outhit (`KismetSystemLibrary.LineTraceSingle` _worldposition (+ _worldposition (* _worlddirection 10000.0)) "TraceTypeQuery1" false (`|MakeArray` _currentcamera :!type "Actor Object Reference") "ForOneFrame" false))
    (bind _asbp_player_camera (cast `/Game/MyContent/BP_Player_Camera` (`.HitActor` (`GameplayStatics.BreakHitResult` _outhit)))
      (:`then`
        (set `self.CurrentTracedCamera` _asbp_player_camera)
        (`self.ShowChangeViewHint` true))
      (:`CastFailed`
        (`self.ShowChangeViewHint` false)))))

(event `Key|R`
  (params (Key :type "Key Structure"))
  (bind _returnvalue (`GameplayStatics.GetPlayerController` 0))
  (bind _currenttracedcamera (`self.CurrentTracedCamera`))
  (:`Pressed`
    (if (`self.CanChangeCamera`)
      (`self.SetViewTargetWithBlend` _returnvalue _currenttracedcamera 1.0 "VTBlend_Linear" 0.0 true)
      (`KismetSystemLibrary.Delay` 1.0)
      (`self.Possess` _returnvalue _currenttracedcamera)
      (set `self.CurrentCamera` (`self.CurrentTracedCamera`)))))

(event `Key|F`
  (params (Key :type "Key Structure"))
  (bind _returnvalue (`GameplayStatics.GetPlayerController` 0))
  (bind _chatuiref (`self.ChatUIRef`))
  (:`Pressed`
    (if (not (`self.ChatOpen`))
      (`/Engine/EditorBlueprintResources/StandardMacros.IsValid` (`self.ChatUIRef`)
        (:`Is Valid`
          (`Widget.SetVisibility` _chatuiref "Visible"))
        (:`Is Not Valid`
          (bind _returnvalue_2 (`|CreateWidget` "/Game/MyContent/WBP_ChatUI.WBP_ChatUI_C"))
          (bind _output_get (set `self.ChatUIRef` _returnvalue_2))
          (`UserWidget.AddToViewport` _output_get 0)))
      (`WidgetBlueprintLibrary.SetInputMode_UIOnlyEx` _returnvalue (`/Game/MyContent/WBP_ChatUI.InputBox` _chatuiref))
      (set `PlayerController.bShowMouseCursor` true _returnvalue)
      (set `self.ChatOpen` true))))

(event `AddChatHistory`
  (params (newMssage :type "AIMessage Structure (by ref)"))
  (bind _asglobal_game_instance (cast `GlobalGameInstance` (`GameplayStatics.GetGameInstance`)))
  (bind _returnvalue (`GlobalGameInstance.GetGPTManager` _asglobal_game_instance))
  (`KismetArrayLibrary.Array_Insert` (`GPTManager.ChatHistory` _returnvalue) newMssage))

(event `SendMessageToLLM`
  (bind _asglobal_game_instance (cast `GlobalGameInstance` (`GameplayStatics.GetGameInstance`)))
  (bind _returnvalue (`GlobalGameInstance.GetGPTManager` _asglobal_game_instance))
  (`GPTManager.SendMessageWithContext` _returnvalue "" (`GPTManager.ChatHistory` _returnvalue) ""))

(fn `UserConstructionScript`)